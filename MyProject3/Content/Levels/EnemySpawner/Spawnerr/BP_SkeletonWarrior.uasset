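; BP_SkeletonWarrior is a skeleton warrior enemy pawn that reacts to seeing the player.
; On BeginPlay it issues a single AI move toward a random reachable point near itself, with an acceptance radius larger than the search radius.
; When PawnSensing spots a BP_TopDownCharacter, it sets the HasSeenPlayer flag on its AI controller's blackboard.
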(event OnSeePawn(PawnSensing)
  (params (Pawn :type Pawn%20Object%20Reference))
  (Utilities|Casting|CastToBP_TopDownCharacter Pawn)
  (AI|Components|Blackboard|SetValueasBool (AI|GetBlackboard (AI|GetAIController self)) (Utilities|Name|MakeLiteralName "HasSeenPlayer") true))

(event Custom|Move
  (AI|AIMoveTo self (.RandomLocation (AI|Navigation|GetRandomReachablePointinRadius (Transformation|GetActorLocation) 1.2e+02 0 0)) 0 3e+02 false))

(event EventBeginPlay
  (CallFunction|Move))

(fn ConstructionScript)